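; OpenStreetMap map actor that turns imported way data into spline roads in the world.
; Its DrawMap override scales the map plane from the map's size in meters, then walks the Ways, converting node coordinates through Projection.EarthToWorld.
; Highways spawn BP_RoadSpline actors with node-based spline points, refreshing spline meshes as points beyond the second are added.
; Other ways only attempt a single debug line each, before the parent DrawMap runs.
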(event EventBeginPlay
  (|CallParentFunction))

(event EventActorBeginOverlap
  (params (OtherActor :type Actor%20Object%20Reference)))

(event EventTick
  (params (DeltaSeconds :type Float%20%28single-precision%29)))

(fn ConstructionScript
  (|CallParentFunction))

(fn DrawMap
  (bind _size (CallFunction|GetSizeMeters))
  (bind _ways (Variables|Default|GetWays))
  (bind (_x _y) (Math|Vector|BreakVector _size))
  ;[1 1 1] Set the Map Mesh to the proper real-world scale
  (Transformation|SetWorldScale3D (Variables|Default|GetMapPlaneMesh) (Math|Vector|MakeVector (/ (* _x 1.0) 1e+03) (/ (* _y 1.0) 1e+03) 1.0))
  (for _index (range 0 (- (Utilities|Array|Length _ways) 1))
    (if (and true (.bIsHighway (Utilities|Struct|BreakOpenStreetWay (Utilities|Array|Get(acopy) _ways _index)))) ; If a highway, make a spline. If not, draw a debug line
      (bind _returnvalue (Game|SpawnActorfromClass "/Game/Blueprints/BP_RoadSpline.BP_RoadSpline_C" (Math|Transform|MakeTransform (Class|MapProjectionComponent|EarthtoWorld (Variables|Default|GetProjection) (.Location (Utilities|Struct|BreakOpenStreetNode (Utilities|Array|Get(acopy) (.Nodes (Utilities|Struct|BreakOpenStreetWay (Utilities|Array|Get(acopy) _ways _index)))))))) "Undefined" 0 0))
      (Spline|SetLocationatSplinePoint (Variables|/Game/Blueprints/BP_RoadSpline.BP_RoadSpline_C|GetSpline _returnvalue) 0 (Class|MapProjectionComponent|EarthtoWorld (Variables|Default|GetProjection) (.Location (Utilities|Struct|BreakOpenStreetNode (Utilities|Array|Get(acopy) (.Nodes (Utilities|Struct|BreakOpenStreetWay (Utilities|Array|Get(acopy) _ways _index))))))) "Local")
      (Spline|SetLocationatSplinePoint (Variables|/Game/Blueprints/BP_RoadSpline.BP_RoadSpline_C|GetSpline _returnvalue) 1 (Class|MapProjectionComponent|EarthtoWorld (Variables|Default|GetProjection) (.Location (Utilities|Struct|BreakOpenStreetNode (Utilities|Array|Get(acopy) (.Nodes (Utilities|Struct|BreakOpenStreetWay (Utilities|Array|Get(acopy) _ways _index))))))) "Local")
      ;[1 1 1] Add the rest of the spline points at the rest of the Nodes
      (if (> (Utilities|Array|Length (.Nodes (Utilities|Struct|BreakOpenStreetWay (Utilities|Array|Get(acopy) _ways _index)))) 2) ; If there are any more points to add
        (for _index_2 (range 2 (- (Utilities|Array|Length (.Nodes (Utilities|Struct|BreakOpenStreetWay (Utilities|Array|Get(acopy) _ways _index)))) 1))
          (Spline|AddSplinePoint (Variables|/Game/Blueprints/BP_RoadSpline.BP_RoadSpline_C|GetSpline _returnvalue) (Class|MapProjectionComponent|EarthtoWorld (Variables|Default|GetProjection) (.Location (Utilities|Struct|BreakOpenStreetNode (Utilities|Array|Get(acopy) (.Nodes (Utilities|Struct|BreakOpenStreetWay (Utilities|Array|Get(acopy) _ways _index))) _index_2)))) "Local")
          (Default|UpdateSplineMeshes _returnvalue)))
      (else
        ;[1 1 1] Draw Debug Line for non-highways
        (if (< _index (- (Utilities|Array|Length (.Nodes (Utilities|Struct|BreakOpenStreetWay (Utilities|Array|Get(acopy) _ways _index)))) 1))
          (Rendering|Debug|DrawDebugLine (Class|MapProjectionComponent|EarthtoWorld (Variables|Default|GetProjection) (.Location (Utilities|Struct|BreakOpenStreetNode (Utilities|Array|Get(acopy) (.Nodes (Utilities|Struct|BreakOpenStreetWay (Utilities|Array|Get(acopy) _ways _index))))))) (Class|MapProjectionComponent|EarthtoWorld (Variables|Default|GetProjection) (.Location (Utilities|Struct|BreakOpenStreetNode (Utilities|Array|Get(acopy) (.Nodes (Utilities|Struct|BreakOpenStreetWay (Utilities|Array|Get(acopy) _ways _index))) (- _index 1))))) (Math|Conversions|ToLinearColor(Color) (Variables|Default|GetDefaultWayColor)) -1.0 (Variables|Default|GetRoadWidth))))))
  (|CallParentFunction))