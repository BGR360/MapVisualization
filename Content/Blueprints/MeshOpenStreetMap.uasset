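; MeshOpenStreetMap is an OpenStreetMap actor that sizes a map plane mesh to the geographic area covered by its projection.
; GetSizeMeters converts the projection's lower-left and upper-right bounds to world space and returns their X/Y difference, which BeginPlay caches as MapSize.
; DrawDebugMap scales MapPlaneMesh from that extent and the projection's scale factor, then defers to the parent's debug drawing.
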(event EventBeginPlay
  (|CallParentFunction)
  (Variables|Default|SetMapSize (Projection|GetSizeMeters)))

(event EventActorBeginOverlap
  (params (OtherActor :type Actor%20Object%20Reference)))

(event EventTick
  (params (DeltaSeconds :type Float%20%28single-precision%29)))

(fn ConstructionScript)

(fn DrawDebugMap
  (bind _size (Projection|GetSizeMeters))
  (bind _projection (Variables|Default|GetProjection))
  (bind (_x _y) (Math|Vector|BreakVector _size))
  (bind _scalefactor (Variables|/Script/MapVisualization.MapProjectionComponent|GetScaleFactor _projection))
  (Transformation|SetWorldScale3D (Variables|Default|GetMapPlaneMesh) (Math|Vector|MakeVector (/ (* _x _scalefactor) 1e+03) (/ (* _y _scalefactor) 1e+03) 1.0))
  (|CallParentFunction))

(fn GetSizeMeters
  (bind _projection (Variables|Default|GetProjection))
  (bind _projection_2 (Variables|Default|GetProjection))
  (bind _projection_3 (Variables|Default|GetProjection))
  (bind _returnvalue (Class|MapProjectionComponent|GetBounds _projection))
  (bind (_lowerleft _upperright) (Utilities|Struct|BreakLatLngBounds _returnvalue))
  (bind _returnvalue_2 (Class|MapProjectionComponent|EarthtoWorld _projection_2 _lowerleft))
  (bind _returnvalue_3 (Class|MapProjectionComponent|EarthtoWorld _projection_3 _upperright))
  (bind (_x _y) (Math|Vector|BreakVector _returnvalue_2))
  (bind (_x_2 _y_2) (Math|Vector|BreakVector _returnvalue_3))
  (return (Math|Vector|MakeVector (- _x_2 _x) (- _y_2 _y) 0.0)))