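; BP_DebugOpenStreetMap is a debug OpenStreetMap actor that shows map data over a tiled grass ground plane.
; Its construction script sets the projection scale factor and way and road colors.
; DrawMap scales the plane from the projected bounds to real-world size, then calls the parent's drawing.
; On BeginPlay it applies a dynamic grass material to the plane, with tiling driven by the projection scale factor.
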(event EventActorBeginOverlap
  (params (OtherActor :type Actor%20Object%20Reference)))

(event EventBeginPlay
  (bind _returnvalue (Rendering|Material|CreateDynamicMaterialInstance (Utilities|Array|Get(acopy) (Rendering|Material|GetMaterials (Variables|Default|GetMapPlaneMesh))) "/Game/Materials/M_Tiled_Grass.M_Tiled_Grass" :!class /Script/Engine.KismetMaterialLibrary))
  (Rendering|Material|SetMaterial (Variables|Default|GetMapPlaneMesh) 0 _returnvalue)
  (Rendering|Material|SetScalarParameterValue _returnvalue "Tiling" (Variables|/Script/MapVisualization.MapProjectionComponent|GetScaleFactor (Variables|Default|GetProjection)) :!class /Script/Engine.MaterialInstanceDynamic))

(event EventTick
  (params (DeltaSeconds :type Float%20%28single-precision%29)))

(fn ConstructionScript
  (Variables|/Script/MapVisualization.MapProjectionComponent|SetScaleFactor (Variables|Default|GetProjection) 1e+02)
  (Variables|Default|SetDefaultWayColor (Math|Color|MakeColor 255 0 255))
  (Variables|Default|SetRoadColor (Math|Color|MakeColor 128 255 32)))

(fn GetSizeMeters
  (bind _projection (Variables|Default|GetProjection))
  (bind _projection_2 (Variables|Default|GetProjection))
  (bind _projection_3 (Variables|Default|GetProjection))
  (bind _returnvalue (Class|MapProjectionComponent|GetBounds _projection))
  (bind (_lowerleft _upperright) (Utilities|Struct|BreakLatLngBounds _returnvalue))
  (bind _returnvalue_2 (Class|MapProjectionComponent|EarthtoWorld _projection_2 _lowerleft))
  (bind _returnvalue_3 (Class|MapProjectionComponent|EarthtoWorld _projection_3 _upperright))
  (bind (_x _y) (Math|Vector|BreakVector _returnvalue_2))
  (bind (_x_2 _y_2) (Math|Vector|BreakVector _returnvalue_3))
  (return (Math|Vector|MakeVector (- _x_2 _x) (- _y_2 _y) 0.0)))

(fn DrawMap
  (bind _size (Projection|GetSizeMeters))
  (bind (_x _y) (Math|Vector|BreakVector _size))
  ;[1 1 1] Set the Map Mesh to the proper real-world scale
  (Transformation|SetWorldScale3D (Variables|Default|GetMapPlaneMesh) (Math|Vector|MakeVector (/ (* _x 1.0) 1e+03) (/ (* _y 1.0) 1e+03) 1.0))
  (|CallParentFunction))