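; BP_RoadSpline is a spline-based road actor whose construction script calls UpdateSplineMeshes and disables actor tick.
; UpdateSplineMeshes loops over each segment between consecutive spline points, but the loop body is empty, so it builds nothing.
; Disconnected nodes would add a spline mesh component per segment, fitted to the local positions and tangents of its two endpoints.
; The event graph has no gameplay logic.
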(event EventBeginPlay)

(event EventActorBeginOverlap
  (params (OtherActor :type Actor%20Object%20Reference)))

(fn ConstructionScript
  (CallFunction|UpdateSplineMeshes)
  (Actor|Tick|SetActorTickEnabled false))

(fn UpdateSplineMeshes
  (for _index (range 0 (- (Spline|GetNumberOfSplinePoints (Variables|Default|GetSpline)) 2))
    _))